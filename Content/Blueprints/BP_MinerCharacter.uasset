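; BP_MinerCharacter is a miner character that moves under AI control and can hold a tool in its right hand.
; Equip spawns the tool from its ToolComponent and attaches it to the hand socket, and un-equip destroys it.
; Block requests drive AIMoveTo, with ArrivedToPlace reporting success, or failure if the move fails or the block is gone.
; It can also walk back to its location saved at BeginPlay.
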(event EventEquipTool
  ;[1 1 1] Equip / Un-equip tool
  (bind _returnvalue (Game|SpawnActorfromClass (Variables|Default|GetTool) (Transformation|GetSocketTransform (Variables|Character|GetMesh) (Variables|Default|GetRightHandSocket) "RTS_World") "AlwaysSpawn" 0 0))
  (bind _output_get (Variables|Default|SetInHandToolActor _returnvalue))
  (Transformation|AttachComponentToComponent _output_get (Variables|Character|GetMesh) (Variables|Default|GetRightHandSocket) "SnapToTarget" "SnapToTarget" "SnapToTarget" true))

(event EventBeginPlay
  (Variables|Default|SetMiner self)
  (Variables|Default|SetTool (Variables|/Script/MCR_Project.MinerCharacter|GetToolComponent (Variables|Default|GetMiner)))
  (Variables|Default|SetStartingLocation (Transformation|GetActorLocation)))

(event EventUnEquipTool
  (bind _inhandtoolactor (Variables|Default|GetInHandToolActor))
  ;[1 1 1] Equip / Un-equip tool
  (Utilities|IsValid _inhandtoolactor
    (:Is%20Valid
      (Actor|DestroyActor _inhandtoolactor))))

(event EventGoBaktoStart
  ;[0.5666 0.6003 0.7083] Movement
  (AI|AIMoveTo (AI|GetAIController self) (Variables|Default|GetStartingLocation) 0 -1.0 "Default" "Default" true true))

(event EventGotoBlockfromRequest
  (params (Request :type Mining%20Request%20Object%20Reference))
  ;[0.5666 0.6003 0.7083] Movement
  (Class|NavMovementComponent|StopActiveMovement (Variables|Character|GetCharacterMovement))
  (bind _returnvalue (Class|MiningRequest|GetBlock Request))
  (AI|AIMoveTo (AI|GetAIController self) "0, 0, 0" _returnvalue 1.5e+02 "Default" "Default" true true
    (:OnRequestFailed
      (Development|PrintString "Miner failed to move to place")
      (Class|MinerCharacter|ArrivedtoPlace Request 0 false :!label _label))
    (:OnMoveFinished
      (Utilities|IsValid _returnvalue
        (:Is%20Valid
          (Class|MinerCharacter|ArrivedtoPlace Request _returnvalue true))
        (:Is%20Not%20Valid
          (Development|PrintString "Place not existing anymore")
          (goto _label))))))

(fn ConstructionScript)

(fn GetToolActor
  (bind _inhandtoolactor (Variables|Default|GetInHandToolActor))
  (Utilities|IsValid _inhandtoolactor
    (:Is%20Valid
      _)
    (:Is%20Not%20Valid
      (Development|PrintString "BP_MinerCharacter: GetToolActor, warning invalid tool")))
  (return _inhandtoolactor))