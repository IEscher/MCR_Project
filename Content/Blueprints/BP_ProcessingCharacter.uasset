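; BP_ProcessingCharacter is an AI-moved worker character that records its spawn location on BeginPlay and can walk back to it through GoBaktoStart.
; GotoBlockfromRequest only stops active movement and ignores the request it receives.
; Tool equipping on the right-hand socket and the move-to-place logic reporting through ArrivedToPlace are unwired and never run.
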(event EventBeginPlay
  (Variables|Default|SetStartingLocation (Transformation|GetActorLocation)))

(event EventGoBaktoStart
  ;[0.5666 0.6003 0.7083] Movement
  (AI|AIMoveTo (AI|GetAIController self) (Variables|Default|GetStartingLocation) 0 -1.0 "Default" "Default" true true))

(event EventGotoBlockfromRequest
  (params (Request :type Mining%20Request%20Object%20Reference))
  ;[0.5666 0.6003 0.7083] Movement
  (Class|NavMovementComponent|StopActiveMovement (Variables|Character|GetCharacterMovement)))

(fn ConstructionScript)